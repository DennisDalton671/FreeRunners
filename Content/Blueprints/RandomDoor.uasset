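; RandomDoor is an actor that keeps one of two doors at random each time play begins.
; On BeginPlay, ChooseDoor flips a random coin into RemoveDoorOne, and the actor destroys either Door1 with PointLight2 or Door2 with PointLight.
; The choice is made at runtime, as the construction script is empty.
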(event `self.ReceiveBeginPlay`
  (`self.ChooseDoor`)
  (if (`self.RemoveDoorOne`)
    (`ActorComponent.K2_DestroyComponent` (`self.Door1`))
    (`ActorComponent.K2_DestroyComponent` (`self.PointLight2`))
    (else
      (`ActorComponent.K2_DestroyComponent` (`self.Door2`))
      (`ActorComponent.K2_DestroyComponent` (`self.PointLight`)))))

(event `ChooseDoor`
  (set `self.RemoveDoorOne` (== (`KismetMathLibrary.RandomInteger` 2) 1)))

(fn `UserConstructionScript`)