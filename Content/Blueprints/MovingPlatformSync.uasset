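; MovingPlatformSync is a moving platform that travels between a start and an end location using an InterpToMovement component.
; The construction script builds two relative control points from those locations and applies the Duration variable to the component.
; StartObject extends the parent's version by activating the movement component without a reset.
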(fn `StartObject`
  (`parent.StartObject`)
  (`ActorComponent.Activate` (`self.InterpToMovement`) false))

(fn `UserConstructionScript`
  (bind _interptomovement (`self.InterpToMovement`))
  (`parent.UserConstructionScript`)
  (set `InterpToMovementComponent.ControlPoints` (`|MakeArray` (make `InterpControlPoint` (`self.StartLocation`)) (make `InterpControlPoint` (`self.EndLocation`))) _interptomovement)
  (set `InterpToMovementComponent.Duration` (`self.Duration`) _interptomovement))