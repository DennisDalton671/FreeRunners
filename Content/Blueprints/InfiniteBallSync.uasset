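; InfiniteBallSync is a self-replacing actor that keeps respawning in a timed loop.
; Tick runs a Delay and then destroys the actor.
; On Destroyed it spawns a new InfiniteBallSync at its root component's relative transform.
; The StartObject override calls the parent and sets StartDelay, which this Blueprint's own graphs never read.
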(event `self.ReceiveTick`
  (params (DeltaSeconds :type "Float (single-precision)"))
  (`KismetSystemLibrary.Delay` (`self.Delay`))
  (`self.K2_DestroyActor`))

(event `self.ReceiveDestroyed`
  (`|SpawnActorFromClass` "InfiniteBallSync_C" (`SceneComponent.GetRelativeTransform` (`self.DefaultSceneRoot`)) "Undefined" "OverrideRootScale" null null))

(fn `StartObject`
  (`parent.StartObject`)
  (set `self.StartDelay` true))

(fn `UserConstructionScript`
  (`parent.UserConstructionScript`))