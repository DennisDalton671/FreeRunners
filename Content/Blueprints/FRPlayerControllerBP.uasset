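; Player controller that handles match start, interaction and the pause menu toggle.
; T asks the game mode to start the match when the game instance reports being in a level, and Use fires ServerInteract, which messages the player state's InteractTarget with the pawn.
; Escape or Y toggles the game instance between Playing and MainMenu states, switching cursor and input mode.
; An unconnected ResetLevel call never runs.
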(event `Key|T`
  (params (Key :type "Key Structure"))
  ;[1 1 1] Start Match
  (:`Pressed`
    (bind _asfrgame_instance_bp (cast `/Game/Blueprints/FRGameInstanceBP` (`GameplayStatics.GetGameInstance`)))
    (`/Game/Blueprints/FRGameInstanceBP.CheckInLevel` _asfrgame_instance_bp)
    (if (`/Game/Blueprints/FRGameInstanceBP.inLevel` _asfrgame_instance_bp)
      (bind _asfrgame_mode_bp (cast `/Game/Blueprints/FRGameModeBP` (`GameplayStatics.GetGameMode`)))
      (`GameMode.StartMatch` _asfrgame_mode_bp))))

(event `InputAction|Restart`
  (params (Key :type "Key Structure")))

(event `InputAction|Use`
  (params (Key :type "Key Structure"))
  ;[1 1 1] interact
  (:`Pressed`
    (`self.ServerInteract`)))

(event `Key|Escape`
  (params (Key :type "Key Structure"))
  ;[1 1 1] Pause
  (:`Pressed`
    (bind _asfrgame_instance_bp (cast `/Game/Blueprints/FRGameInstanceBP` (`GameplayStatics.GetGameInstance`) :!label _label))
    (if (`self.inMenu`)
      (`FRGameInstance.TransitionToState` _asfrgame_instance_bp "Playing")
      (set `self.inMenu` false)
      (set `PlayerController.bShowMouseCursor` false)
      (`WidgetBlueprintLibrary.SetInputMode_GameOnly` self)
      (else
        (`FRGameInstance.TransitionToState` _asfrgame_instance_bp "MainMenu")
        (set `self.inMenu` true)
        (set `PlayerController.bShowMouseCursor` true)
        (`WidgetBlueprintLibrary.SetInputMode_GameAndUIEx` self (`FRGameInstance.MainMenuWidget` _asfrgame_instance_bp) "DoNotLock" false)))))

(event `ServerInteract`
  (bind _playerstate (`Controller.PlayerState`))
  ;[1 1 1] interact
  (bind _asfrplayer_state_bp (cast `/Game/Blueprints/FRPlayerStateBP` _playerstate))
  (message `/Game/Blueprints/FRInterface.Interact` (`/Game/Blueprints/FRPlayerStateBP.InteractTarget` _asfrplayer_state_bp) (`PlayerState.PawnPrivate` _playerstate)))

(event `Key|Y`
  (params (Key :type "Key Structure"))
  ;[1 1 1] Pause
  (:`Pressed`
    (goto _label)))

(fn `UserConstructionScript`)