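; InfiniteBalls is an actor that endlessly recycles itself on a five-second cycle.
; Tick waits on a Delay and then destroys the actor, and the Destroyed event spawns a fresh InfiniteBalls at the root component's transform.
; A SetBallTimer event can write Seconds to the LevelSelector game instance's BallTimer once, gated by Check, but its only call in this graph never runs.
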(event `Set Ball Timer`
  (if (`self.Check`)
    (bind _aslevel_selector (cast `/Game/UI/LevelSelector` (`GameplayStatics.GetGameInstance`)))
    (set `/Game/UI/LevelSelector.BallTimer` (`self.Seconds`) _aslevel_selector)
    (set `self.Check` false)))

(event `self.ReceiveBeginPlay`)

(event `self.ReceiveTick`
  (params (DeltaSeconds :type "Float (single-precision)"))
  (`KismetSystemLibrary.Delay` 5.0)
  (`self.K2_DestroyActor`))

(event `self.ReceiveDestroyed`
  (`|SpawnActorFromClass` "InfiniteBalls_C" (`SceneComponent.GetRelativeTransform` (`self.DefaultSceneRoot`)) "Undefined" "OverrideRootScale" null null))

(fn `UserConstructionScript`)