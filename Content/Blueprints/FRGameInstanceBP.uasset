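; Game instance that owns the front-end UI and tracks the game's current state across menus, loading and play.
; Init creates and caches the menu, loading and play UI widgets; named events request screen changes through TransitionToState, and LoadLevel opens a level before switching to Playing.
; IsCurrentState branches logic: returning to the menu from play reloads the MainMenu level, and CheckInLevel treats Playing or Startup as in-level.
; Leaving a game destroys the session, then goes to the main menu.
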(event `self.ReceiveInit`
  (bind _returnvalue (`GameplayStatics.GetPlayerController` 0))
  ;[1 1 1] create widgets
  (bind _returnvalue_2 (`|CreateWidget` "/Game/UI/MainMenu.MainMenu_C" _returnvalue))
  (set `self.MainMenuWidget` _returnvalue_2)
  (bind _returnvalue_3 (`|CreateWidget` "/Game/UI/LoadingScreen.LoadingScreen_C" _returnvalue))
  (set `self.LoadingWidget` _returnvalue_3)
  (bind _returnvalue_4 (`|CreateWidget` "/Game/UI/MainMenu_Multiplayer.MainMenu_Multiplayer_C" _returnvalue))
  (set `self.MultiplayerWidget` _returnvalue_4)
  (bind _returnvalue_5 (`|CreateWidget` "/Game/UI/MainMenu_Settings.MainMenu_Settings_C" _returnvalue))
  (set `self.SettingsWidget` _returnvalue_5)
  (bind _returnvalue_6 (`|CreateWidget` "/Game/UI/Play_UI.Play_UI_C" _returnvalue))
  (set `self.PlayUIWidget` _returnvalue_6)
  (bind _returnvalue_7 (`|CreateWidget` "/Game/UI/MainMenu_LevelSelect.MainMenu_LevelSelect_C" _returnvalue))
  (set `self.LevelSelectWidget` _returnvalue_7))

(event `LoadLevel`
  (params (`Level Name` :type Name) (Options :type String))
  ;[1 1 1] loads a level w/ options and transitions to playing state
  (`GameplayStatics.OpenLevel` `Level Name` true Options)
  (`self.TransitionToState` "Playing"))

(event `ShowMultiplayer`
  ;[1 1 1] show multiplayer
  (`self.TransitionToState` "Multiplayer"))

(event `ShowLoadingScreen`
  ;[1 1 1] show loading screen
  (`self.TransitionToState` "Loading"))

(event `GotoMainMenu`
  ;[1 1 1] goto main menu (level if in gameplay)
  (`self.IsCurrentState` "Playing"
    (:`True`
      (`GameplayStatics.OpenLevel` "MainMenu"))
    (:`False`
      (`self.TransitionToState` "MainMenu"))))

(event `ShowLevelSelect`
  ;[1 1 1] show level select
  (`self.TransitionToState` "LevelSelect"))

(event `ShowSettings`
  ;[1 1 1] show settings
  (`self.TransitionToState` "Settings"))

(event `self.DestroyOrLeaveGame`
  ;[1 1 1] destroy or leave session
  (`DestroySessionCallbackProxy.DestroySession` (`GameplayStatics.GetPlayerController` 0)
    (:`then`
      _)
    (:`OnSuccess`
      _))
  (`self.GotoMainMenu`))

(event `CheckInLevel`
  ;[1 1 1] LevelCheck
  (`self.IsCurrentState` "Playing"
    (:`True`
      (set `self.inLevel` true :!label _label))
    (:`False`
      (`self.IsCurrentState` "Startup"
        (:`True`
          (goto _label))
        (:`False`
          (set `self.inLevel` false))))))

(event `SetStateMenu`
  ;[1 1 1] Set State To Menu
  (set `self.CurrentState` "MainMenu"))