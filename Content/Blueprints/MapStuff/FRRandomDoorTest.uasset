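; A test map object that randomly removes one of its two doors, leaving the other in place.
; When the inherited StartObject event runs, the authority rolls a roughly even chance and passes the result to DestroyDoor.
; DestroyDoor destroys either Door1 with PointLight2 or Door2 with PointLight, so each door is removed alongside the oppositely numbered light.
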(event `self.ReceiveBeginPlay`
  (`parent.ReceiveBeginPlay`))

(event `self.StartObject`
  (`parent.StartObject`)
  (`/Engine/EditorBlueprintResources/ActorMacros.Switch Has Authority`
    (:`Authority`
      (bind _output_get (set `self.RemoveDoorOne` (>= (`KismetMathLibrary.RandomInteger` 100) 49)))
      (`self.DestroyDoor` _output_get))))

(event `DestroyDoor`
  (params (DoorOne :type Boolean))
  (if DoorOne
    (`ActorComponent.K2_DestroyComponent` (`self.Door1`))
    (`ActorComponent.K2_DestroyComponent` (`self.PointLight2`))
    (else
      (`ActorComponent.K2_DestroyComponent` (`self.Door2`))
      (`ActorComponent.K2_DestroyComponent` (`self.PointLight`)))))

(fn `UserConstructionScript`)