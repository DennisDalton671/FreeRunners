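; EndGoal is the level's finish trigger, which shows the player's time and the end-of-game screen when an actor overlaps it.
; On overlap, unless Completed is already visible, it takes the time text from FRGameStateBP and toggles the Time and Completed components on.
; After a short delay it toggles them again, adds the EndOfGameBP widget to the viewport and shows the mouse cursor.
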(event `self.ReceiveActorBeginOverlap`
  (params (OtherActor :type "Actor Object Reference"))
  (bind _completed (`self.Completed`))
  (bind _time (`self.Time`))
  (if (not (`SceneComponent.IsVisible` (`self.Completed`)))
    (bind _asfrgame_state_bp (cast `/Game/Blueprints/FRGameStateBP` (`GameplayStatics.GetGameState`)))
    (bind _returnvalue (`FRGameState.GetTimeAsText` _asfrgame_state_bp))
    (`TextRenderComponent.K2_SetText` _time _returnvalue)
    (`SceneComponent.ToggleVisibility` _time false)
    (`SceneComponent.ToggleVisibility` _completed false)
    (`KismetSystemLibrary.Delay` 3.0)
    (`SceneComponent.ToggleVisibility` _completed false)
    (`SceneComponent.ToggleVisibility` _time false)
    (bind _returnvalue_2 (`|CreateWidget` "/Game/UI/EndOfGameBP.EndOfGameBP_C"))
    (`UserWidget.AddToViewport` _returnvalue_2 0)
    (set `PlayerController.bShowMouseCursor` true (`GameplayStatics.GetPlayerController` 0))))

(fn `UserConstructionScript`)