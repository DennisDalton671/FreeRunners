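; Map actor with two door and light options that is meant to keep one at random.
; On BeginPlay the authority sets RemoveDoorOne from a random integer, though a max of 1 always yields false.
; A separate StartObject event reads the flag and destroys either Door1 with PointLight2 or Door2 with PointLight, so as written Door1 remains wherever the flag comes from that roll.
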(event `self.ReceiveBeginPlay`
  (`/Engine/EditorBlueprintResources/ActorMacros.Switch Has Authority`
    (:`Authority`
      (set `self.RemoveDoorOne` (`KismetMathLibrary.Conv_IntToBool` (`KismetMathLibrary.RandomInteger` 1))))))

(event `self.StartObject`
  (if (`self.RemoveDoorOne`)
    (`ActorComponent.K2_DestroyComponent` (`self.Door1`))
    (`ActorComponent.K2_DestroyComponent` (`self.PointLight2`))
    (else
      (`ActorComponent.K2_DestroyComponent` (`self.Door2`))
      (`ActorComponent.K2_DestroyComponent` (`self.PointLight`)))))

(fn `UserConstructionScript`)