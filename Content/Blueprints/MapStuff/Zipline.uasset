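; Zipline actor that carries an interacting actor along a spline when that actor overlaps its trigger.
; The construction script builds spline mesh segments between spline points and positions start and end components at the spline's ends.
; A timeline, with play rate set on BeginPlay, sweeps the rider along the spline at a fixed offset below it.
; A DoOnce blocks new rides until the current one finishes.
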(event `/Game/Blueprints/FRInterface.Interact`
  (params (Instigator :type "Actor Object Reference"))
  ;[1 1 1] zipline interact; check if in trigger before doing movement
  (if (`PrimitiveComponent.IsOverlappingActor` (`self.Trigger`) Instigator)
    (`self.ZiplineMovement` Instigator)))

(event `self.ReceiveBeginPlay`
  ;[1 1 1] setup zipline
  (`TimelineComponent.SetPlayRate` (`self.ZipTime`) (`self.PlayRate`)))

(event `ZiplineMovement`
  (params (Actor :type "Actor Object Reference"))
  ;[1 1 1] zipline movement
  (`/Engine/EditorBlueprintResources/StandardMacros.DoOnce` false :!label _label
    (:`Completed`
      (bind (_direction _movement) (`Timeline|ZipTime` :`NewTime` 0.2 :!via `PlayFromStart`)
        (:`Update`
          (`self.K2_SetActorLocation` Actor (`KismetMathLibrary.MakeVector` (.x (`SplineComponent.GetLocationAtDistanceAlongSpline` (`self.Zipline`) (* _movement (`SplineComponent.GetSplineLength` (`self.Zipline`))) "World")) (.y (`SplineComponent.GetLocationAtDistanceAlongSpline` (`self.Zipline`) (* _movement (`SplineComponent.GetSplineLength` (`self.Zipline`))) "World")) (- (.z (`SplineComponent.GetLocationAtDistanceAlongSpline` (`self.Zipline`) (* _movement (`SplineComponent.GetSplineLength` (`self.Zipline`))) "World")) 120.0)) true false))
        (:`Finished`
          (goto _label :!via `Reset`))))))

(fn `UserConstructionScript`
  (bind _zipline (`self.Zipline`))
  (bind _mesh (`self.Mesh`))
  (bind _zipline_2 (`self.Zipline`))
  (bind _returnvalue (`SplineComponent.GetNumberOfSplinePoints` _zipline_2))
  ;[1 1 1] set start and end points of total spline
  (`SceneComponent.K2_SetRelativeLocation` (`self.End_Point`) (`SplineComponent.GetLocationAtSplinePoint` _zipline_2 _returnvalue "Local") false false)
  (`SceneComponent.K2_SetRelativeLocation` (`self.Start_Point`) (`SplineComponent.GetLocationAtSplinePoint` _zipline_2 0 "Local") false false)
  ;[1 1 1] iterate for every point except start/end
  (for _index (range (+ (- _returnvalue 2) 1))
    ;[1 1 1] setup spline for each segment and attach to the root component
    (bind _returnvalue_2 (`AddComponent|NODE_AddSplineMeshComponent-1`))
    (`SceneComponent.K2_AttachToComponent` _returnvalue_2 (`self.DefaultSceneRoot`) "None" "KeepRelative" "KeepRelative" "KeepRelative" true)
    (bind (_location _tangent) (`SplineComponent.GetLocationAndTangentAtSplinePoint` _zipline _index "Local"))
    (bind (_location_2 _tangent_2) (`SplineComponent.GetLocationAndTangentAtSplinePoint` _zipline (+ _index 1) "Local"))
    (`SplineMeshComponent.SetStartAndEnd` _returnvalue_2 _location _tangent _location_2 _tangent_2 true)
    (`StaticMeshComponent.SetStaticMesh` (`self.Mesh_1`) _mesh)
    (`StaticMeshComponent.SetStaticMesh` (`self.Mesh_2`) _mesh)))