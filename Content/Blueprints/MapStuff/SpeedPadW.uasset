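; Speed pad that temporarily changes the walk speed of a ThirdPersonCharacter that overlaps its box.
; On overlap it stores the current max speed, scales MaxWalkSpeed by SpeedMultiplier, then restores it after a SpeedDuration delay.
; A SpeedModified flag on the character blocks stacking while the effect is active.
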(event `self.Box.OnComponentBeginOverlap`
  (params (OverlappedComponent :type "PrimitiveComponent Object Reference") (OtherActor :type "Actor Object Reference") (OtherComp :type "PrimitiveComponent Object Reference") (OtherBodyIndex :type Integer) (bFromSweep :type Boolean) (SweepResult :type "HitResult Structure (by ref)"))
  (bind _returnvalue (`MovementComponent.GetMaxSpeed` (`self.CharMove`)))
  ;[1 1 1] Speed
  (bind _asthird_person_character (cast `/Game/Blueprints/ThirdPersonCharacter` OtherActor))
  (if (not (`/Game/Blueprints/ThirdPersonCharacter.speedModified` _asthird_person_character))
    (set `/Game/Blueprints/ThirdPersonCharacter.speedModified` true _asthird_person_character)
    (set `self.CharMove` (`Character.CharacterMovement` _asthird_person_character))
    (bind _output_get (set `self.InitalSpeed` _returnvalue))
    (set `CharacterMovementComponent.MaxWalkSpeed` (* _returnvalue (`self.SpeedMultiplier`)) (`self.CharMove`))
    (`KismetSystemLibrary.Delay` (`self.SpeedDuration`))
    (set `CharacterMovementComponent.MaxWalkSpeed` _output_get (`self.CharMove`))
    (set `/Game/Blueprints/ThirdPersonCharacter.speedModified` false _asthird_person_character)))

(fn `UserConstructionScript`)