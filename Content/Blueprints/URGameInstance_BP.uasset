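; Game instance Blueprint that drives menu and play flow through a state machine spanning main menu, loading, multiplayer lobbies, level select, settings and play.
; CreateWidgets builds the UI for these screens up front, caching all but the Settings widget.
; TransitionToState rejects same-state changes, removes the old widget or destroys the session when leaving Playing, and adds only the Play UI on entry.
; Events request menu transitions and forward level loads.
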(event `LoadLevels`
  (params (Level :type Name))
  (`self.LoadLevel` Level))

(event `DestroySessionEvent`
  ;[1 1 1] Destroy/Leave session
  (`DestroySessionCallbackProxy.DestroySession` (`GameplayStatics.GetPlayerController` 0)))

(event `ShowMainMenu`
  ;[1 1 1] Shows the main menu and loads the MainMenu level
  (`self.IsCurrentState` "NewEnumerator1"
    (:`True`
      (`GameplayStatics.OpenLevel` "MenuTest"))
    (:`False`
      _))
  (`self.TransitionToState` "NewEnumerator2"))

(event `ShowMultiplayer`
  (`self.TransitionToState` "NewEnumerator4"))

(fn `BeginPlayShowMainMenu`
  (`self.IsCurrentState` "NewEnumerator0"))

(fn `CreateWidgets`
  (bind _returnvalue (`GameplayStatics.GetPlayerController` 0))
  (bind _returnvalue_2 (`|CreateWidget` "/Game/UI/MainMenu.MainMenu_C" _returnvalue))
  (set `self.MainMenu` _returnvalue_2)
  (bind _returnvalue_3 (`|CreateWidget` "/Game/UI/LoadingScreen.LoadingScreen_C" _returnvalue))
  (set `self.LoadingScreen` _returnvalue_3)
  (bind _returnvalue_4 (`|CreateWidget` "/Game/UI/MainMenu_Multiplayer.MainMenu_Multiplayer_C" _returnvalue))
  (set `self.Multiplayer` _returnvalue_4)
  (bind _returnvalue_5 (`|CreateWidget` "/Game/UI/MainMenu_Multiplayer_Lobby.MainMenu_Multiplayer_Lobby_C" _returnvalue))
  (set `self.Lobby` _returnvalue_5)
  (bind _returnvalue_6 (`|CreateWidget` "/Game/UI/Play_UI.Play_UI_C" _returnvalue))
  (set `self.PlayUI` _returnvalue_6)
  (bind _returnvalue_7 (`|CreateWidget` "/Game/UI/MainMenu_LevelSelect.MainMenu_LevelSelect_C" _returnvalue))
  (set `self.LevelSelect` _returnvalue_7)
  (`|CreateWidget` "/Game/UI/MainMenu_Settings.MainMenu_Settings_C" _returnvalue))